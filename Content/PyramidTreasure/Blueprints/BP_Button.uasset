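; BP_Button is a one-shot pressure button that opens a door with a short camera cutaway.
; Any overlap on its Box moves the button mesh to a pressed position, plays a click and destroys the Box to prevent retriggering.
; A delay-timed sequence then switches the view to Camera, plays the LS_Door level sequence with door audio, and returns the view to the player character.
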(event `self.Box.OnComponentBeginOverlap`
  (params (OverlappedComponent :type "PrimitiveComponent Object Reference") (OtherActor :type "Actor Object Reference") (OtherComp :type "PrimitiveComponent Object Reference") (OtherBodyIndex :type Integer) (bFromSweep :type Boolean) (SweepResult :type "HitResult Structure (by ref)"))
  (`SceneComponent.K2_SetRelativeLocationAndRotation` (`self.Button_StaticMesh`) (0.0 0.0 6.8) (struct :`Yaw` 45.0 :`Roll` 90.0) false false)
  (`GameplayStatics.PlaySound2D` "/Game/PyramidTreasure/Audio/A_Button.A_Button" 1.0 1.0 0.0 null null)
  (`ActorComponent.K2_DestroyComponent` (`self.Box`))
  ; ChangeCamera
  (`KismetSystemLibrary.Delay` 0.3)
  (`PlayerController.SetViewTargetWithBlend` (`GameplayStatics.GetPlayerController` 0) (`self.Camera`) 0.0 "VTBlend_Linear" 0.0 false)
  (`KismetSystemLibrary.Delay` 0.3)
  (bind _outactor (`LevelSequencePlayer.CreateLevelSequencePlayer` "/Game/PyramidTreasure/Animation/LS_Door.LS_Door"))
  (`MovieSceneSequencePlayer.Play` (`LevelSequenceActor.SequencePlayer` _outactor))
  (`GameplayStatics.PlaySound2D` "/Game/PyramidTreasure/Audio/A_Door.A_Door" 1.0 1.0 0.0 null null)
  (`KismetSystemLibrary.Delay` 2.0)
  (`PlayerController.SetViewTargetWithBlend` (`GameplayStatics.GetPlayerController` 0) (`GameplayStatics.GetPlayerCharacter` 0) 0.0 "VTBlend_Linear" 0.0 false))

(fn `UserConstructionScript`)